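; BP_BaseCharacter is a character Blueprint that gives its mesh an animated eye blink.
; On BeginPlay it creates a dynamic material instance for the "eyecover" slot, then plays the looping Eyeblink timeline.
; The timeline's Blinkheight track interpolates the material's "height" parameter between BlinkMin and BlinkMax.
; Tick prints the head socket location every frame, apparently as debug output.
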(event `self.ReceiveBeginPlay`
  (bind _mesh (`self.Mesh`))
  (`|ExecutionSequence`
    (:`then_0`
      (bind _returnvalue (`PrimitiveComponent.CreateDynamicMaterialInstance` _mesh (`PrimitiveComponent.GetMaterialIndex` _mesh "eyecover") (`PrimitiveComponent.GetMaterialByName` _mesh "eyecover") "None"))
      (set `self.EyecoverDMI` _returnvalue))
    (:`then_1`
      (`TimelineComponent.SetLooping` (`self.Eyeblink`) true)
      (bind (_direction _blinkheight) (`Timeline|Eyeblink`)
        (:`Update`
          (`MaterialInstanceDynamic.SetScalarParameterValue` (`self.EyecoverDMI`) "height" (+ (`self.BlinkMin`) (* _blinkheight (- (`self.BlinkMax`) (`self.BlinkMin`))))))))
    (:`then_2`)))

(event `self.ReceiveTick`
  (params (DeltaSeconds :type "Float (single-precision)"))
  (`KismetSystemLibrary.PrintString` (`KismetStringLibrary.Conv_VectorToString` (`SceneComponent.GetSocketLocation` (`self.Mesh`) "head"))))

(fn `UserConstructionScript`)