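; BP_Pokemon is a Pokemon actor that drives an eye-blink effect through its mesh material.
; On BeginPlay it creates a dynamic instance of the "eyecover" material slot, if present, and starts the looping EyeBlink timeline.
; Each tick it feeds the neck bone's world position and up vector, plus a height scaled by the blink percentage, into that material, anchoring the cover to the animated head.
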(event `self.ReceiveBeginPlay`
  (bind _eyeblink (`self.EyeBlink`))
  (bind _succeed (`self.CreateEyecover`))
  (if _succeed
    (`TimelineComponent.SetLooping` _eyeblink true)
    (`TimelineComponent.Play` _eyeblink)))

(event `self.ReceiveTick`
  (params (DeltaSeconds :type "Float (single-precision)"))
  (`|ExecutionSequence`
    (:`then_0`
      (`self.ControlEyecover`))))

(fn `ControlEyecover`
  (bind _eyecoverdm (`self.EyecoverDM`))
  (bind (_returnvalue_location _returnvalue_rotation) (`KismetMathLibrary.BreakTransform` (`SkinnedMeshComponent.GetBoneTransform` (`self.Mesh`) "neck" "RTS_World")))
  (`self.EyecoverDM`
    (:`then`
      (`MaterialInstanceDynamic.SetVectorParameterValue` _eyecoverdm "Pivot" (`KismetMathLibrary.Conv_VectorToLinearColor` _returnvalue_location))
      (`MaterialInstanceDynamic.SetVectorParameterValue` _eyecoverdm "UpVector" (`KismetMathLibrary.Conv_VectorToLinearColor` (`KismetMathLibrary.GetUpVector` _returnvalue_rotation)))
      (`MaterialInstanceDynamic.SetScalarParameterValue` _eyecoverdm "Height" (+ (* (`self.EyecoverHeight`) (`self.Percantage`)) (`self.EyecoverMin`))))
    (:`else`)))

(fn `CreateEyecover`
  (returns (Succeed :type Boolean))
  (bind _mesh (`self.Mesh`))
  (bind _returnvalue (`PrimitiveComponent.GetMaterialIndex` _mesh "eyecover"))
  (if (>= _returnvalue 0)
    (bind _returnvalue_2 (`PrimitiveComponent.CreateDynamicMaterialInstance` _mesh _returnvalue (`PrimitiveComponent.GetMaterial` _mesh _returnvalue) "None"))
    (set `self.EyecoverDM` _returnvalue_2)
    (return true)
    (else
      (return false))))

(fn `UserConstructionScript`)